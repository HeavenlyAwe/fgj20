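; Game mode for the flying saucer game, tracking game state, score and pollution, and handling start, restart and quit.
; Score and pollution events write into the NewHud widget; pollution also updates the saucer camera, and reaching the maximum sets a new state, plays a game-over cue and spawns restart and quit actors.
; Menu choices are world actors, placed either side of the saucer by offsetting the yaw of its origin-relative position.
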(event Custom|ChangePollutionEvent
  (params (Value :type Integer))
  (bind _output_get (Variables|Default|SetPollution (+ Value (Variables|Default|GetPollution))))
  (bind _foundwidgets (Widget|GetAllWidgetsOfClass "/Game/Blueprints/NewHud.NewHud_C" true))
  (bind _output_get_2 (Variables|/Game/Blueprints/NewHud.NewHud_C|SetPollution (Utilities|Array|Get(acopy) _foundwidgets) _output_get))
  (bind _returnvalue (Actor|GetActorOfClass "/Game/Blueprints/FlyingSaucerCamera.FlyingSaucerCamera_C"))
  (Default|UpdatePollution _returnvalue _output_get_2 (Variables|Default|GetMaximumPollution))
  (if (== _output_get_2 (Variables|Default|GetMaximumPollution))
    (Variables|Default|SetCurrentGameState "NewEnumerator2")
    (CallFunction|SpawnRestartActor)
    (Audio|Components|Audio|Play (Variables|Default|GetGameOver_cue) 0.0)))

(event Custom|AddScoreEvent
  (bind _result (Math|Integer|IncrementInt (Variables|Default|GetScore))
    (:%20%20
      (bind _foundwidgets (Widget|GetAllWidgetsOfClass "/Game/Blueprints/NewHud.NewHud_C" true))
      (Variables|/Game/Blueprints/NewHud.NewHud_C|SetScore (Utilities|Array|Get(acopy) _foundwidgets) _result))))

(event Custom|RestartGameEvent
  (bind _returnvalue (Game|GetCurrentLevelName true))
  (Game|OpenLevel(byName) (Utilities|String|StringToName _returnvalue)))

(event Custom|StartGameEvent
  (bind _returnvalue (Actor|GetActorOfClass "/Game/Blueprints/MenuActors/StartGameActor.StartGameActor_C"))
  (Actor|DestroyActor _returnvalue)
  (bind _returnvalue_2 (Actor|GetActorOfClass "/Game/Blueprints/MenuActors/QuitGameActor.QuitGameActor_C"))
  (Actor|DestroyActor _returnvalue_2)
  (Variables|Default|SetCurrentGameState "NewEnumerator0"))

(event Custom|QuitGameEvent
  (Game|QuitGame 0 "Quit" false))

(event Custom|SetupStartActorsEvent
  (CallFunction|SpawnStartActor))

(event EventBeginPlay)

(event EventTick
  (params (DeltaSeconds :type Float%20%28single-precision%29)))

(fn ConstructionScript)

(fn SpawnRestartActor
  (bind _returnvalue (Actor|GetActorOfClass "/Game/Blueprints/FlyingSaucer.FlyingSaucer_C"))
  (bind (_transform1 _transform2) (CallFunction|SpawnActorHelper _returnvalue))
  (Game|SpawnActorfromClass "/Game/Blueprints/MenuActors/RestartGameActor.RestartGameActor_C" _transform1 "AlwaysSpawn" 0 0)
  (Game|SpawnActorfromClass "/Game/Blueprints/MenuActors/QuitGameActor.QuitGameActor_C" _transform2 "AlwaysSpawn" 0 0))

(fn SpawnStartActor
  (bind _returnvalue (Actor|GetActorOfClass "/Game/Blueprints/FlyingSaucer.FlyingSaucer_C"))
  (bind (_transform1 _transform2) (CallFunction|SpawnActorHelper _returnvalue))
  (Game|SpawnActorfromClass "/Game/Blueprints/MenuActors/StartGameActor.StartGameActor_C" _transform1 "AlwaysSpawn" 0 0)
  (Game|SpawnActorfromClass "/Game/Blueprints/MenuActors/QuitGameActor.QuitGameActor_C" _transform2 "AlwaysSpawn" 0 0))

(fn SpawnActorHelper
  (params (Reference :type Actor%20Object%20Reference))
  (bind _returnvalue (Transformation|GetActorLocation Reference))
  (bind _returnvalue_2 (Transformation|GetActorUpVector Reference))
  (bind _buttonoffset (Variables|Default|GetButtonOffset))
  (bind _buttonoffset_2 (Variables|Default|GetButtonOffset))
  (bind _returnvalue_3 (* _returnvalue_2 1e+02))
  (bind _returnvalue_4 (- _returnvalue _returnvalue_3))
  (bind _yaw (Math|Vector|GetYawPitchfromVector _returnvalue_4))
  (bind _returnvalue_5 (Math|Vector|VectorLength _returnvalue_4))
  (bind _returnvalue_6 (- _yaw _buttonoffset_2))
  (bind _returnvalue_7 (+ _yaw _buttonoffset))
  (bind _returnvalue_8 (Class|KismetMathLibrary|CreateVectorfromYawPitch _returnvalue_7 0.0 _returnvalue_5))
  (bind _returnvalue_9 (Class|KismetMathLibrary|CreateVectorfromYawPitch _returnvalue_6 0.0 _returnvalue_5))
  (return (Math|Transform|MakeTransform _returnvalue_8 (Math|Rotator|MakeRotfromZ _returnvalue_8) "0.500000,0.500000,0.500000") (Math|Transform|MakeTransform _returnvalue_9 (Math|Rotator|MakeRotfromZ _returnvalue_9) "0.500000,0.500000,0.500000")))