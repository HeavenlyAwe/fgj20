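; TriangleGrid builds a list of triangles from the Continents static mesh of the Earth actor at BeginPlay.
; It reads LOD 0, section 0 with GetSectionFromStaticMesh, then walks the index buffer in steps of three.
; Each step adds a triangle to TriangleList and fills its Corners with the three indexed vertices.
; Index and triangle counts are printed for debugging.
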(event EventBeginPlay
  (bind _returnvalue (Actor|GetActorOfClass "/Game/Blueprints/Earth.Earth_C"))
  (bind (_vertices _triangles) (Class|KismetProceduralMeshLibrary|GetSectionfromStaticMesh (Variables|/Script/Engine.StaticMeshComponent|GetStaticMesh (Variables|/Game/Blueprints/Earth.Earth_C|GetContinents _returnvalue))))
  (Development|PrintString (Utilities|String|ToString(Integer) (Utilities|Array|Length _triangles)))
  (while (< (Variables|Default|GetStep) (- (Utilities|Array|Length _triangles) 3))
    (Variables|Default|SetStep (+ (Variables|Default|GetStep) 3))
    (bind _returnvalue_2 (AddComponent|AddTriangle))
    (Utilities|Array|Add (Variables|Default|GetTriangleList) _returnvalue_2)
    (for _index (range 0 2)
      (Utilities|Array|Insert (Variables|/Game/Blueprints/TreeSpawner/Triangle.Triangle_C|GetCorners _returnvalue_2) (Utilities|Array|Get(acopy) _vertices (Utilities|Array|Get(acopy) _triangles (+ (Variables|Default|GetStep) _index))) _index)))
  (Development|PrintString (Utilities|String|ToString(Integer) (Utilities|Array|Length (Variables|Default|GetTriangleList)))))

(event Collision|EventActorBeginOverlap
  (params (OtherActor :type Actor%20Object%20Reference)))

(event EventTick
  (params (DeltaSeconds :type Float%20%28single-precision%29)))

(fn ConstructionScript)