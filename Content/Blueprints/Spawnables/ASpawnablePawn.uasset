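; Base pawn for objects spawned on the spherical Earth, such as cars and ships that roam its surface, with helpers to change game-mode pollution.
; Each tick it steps forward, line-traces to snap onto the Earth and carries its heading over to the new surface normal.
; Trace distance distinguishes water from ground, so class-name checks turn cars away from water and ships away from land in a random, roughly backward direction.
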(event Custom|EventNewDirection
  ;[1 1 1] Choose random new direction to move in
  (Transformation|SetActorRotation (Math|Transform|TransformRotation (Math|Transform|MakeTransform "0, 0, 0" (Transformation|GetActorRotation)) (Math|Rotator|MakeRotator 0.0 0.0 (Math|Random|RandomFloatinRange 9e+01 2.7e+02)))))

(event EventBeginPlay)

(event Collision|EventActorBeginOverlap
  (params (OtherActor :type Actor%20Object%20Reference)))

(event EventTick
  (params (DeltaSeconds :type Float%20%28single-precision%29))
  (bind _output_get (Variables|Default|Settmp_location (Transformation|GetActorLocation)))
  (CallFunction|SetPositionBots (.Yaw (Math|Vector|GetYawPitchfromVector (+ (* (Transformation|GetActorForwardVector) (* (Variables|Default|GetSpeed) DeltaSeconds)) _output_get))) (.Pitch (Math|Vector|GetYawPitchfromVector (+ (* (Transformation|GetActorForwardVector) (* (Variables|Default|GetSpeed) DeltaSeconds)) _output_get))) (Math|Vector|VectorLength (+ (* (Transformation|GetActorForwardVector) (* (Variables|Default|GetSpeed) DeltaSeconds)) _output_get)))
  ;[1 1 1] Measure distance to earth (from random point in space)
  (bind _outhit (Collision|LineTraceForObjects (* (Math|Vector|Normalize (+ (Transformation|GetActorForwardVector) (Transformation|GetActorLocation))) 550) "0, 0, 0" (Utilities|Array|MakeArray "ObjectTypeQuery1") true 0 "None"))
  (Utilities|Casting|CastToEarth (.HitActor (Collision|BreakHitResult _outhit)))
  (Transformation|SetActorLocation (* (Math|Vector|Normalize (Transformation|GetActorLocation)) (- 5.5e+02 (.Distance (Collision|BreakHitResult _outhit)))) false false)
  (Transformation|SetActorRotation (Math|Transform|TransformRotation (Math|Transform|MakeTransform "0, 0, 0" (Math|Rotator|MakeRotfromZ (* (Math|Vector|Normalize (Transformation|GetActorLocation)) (- 5.5e+02 (.Distance (Collision|BreakHitResult _outhit)))))) (Math|Transform|InverseTransformRotation (Math|Transform|MakeTransform "0, 0, 0" (Math|Rotator|MakeRotfromZ _output_get)) (Transformation|GetActorRotation))))
  (Math|Float|CompareFloat (.Distance (Collision|BreakHitResult _outhit)) 5e+01 ; If larger than 50, on water, else on ground
    (:>
      (if (Utilities|Enum|Equal(Enum) (Utilities|GetClassDisplayName (Utilities|GetClass self)) "Car_C")
        (CallFunction|EventNewDirection)))
    (:<
      (if (Utilities|Enum|Equal(Enum) (Utilities|GetClassDisplayName (Utilities|GetClass self)) "Ship_C")
        (CallFunction|EventNewDirection)))))

(fn ConstructionScript)

(fn AddPollution
  (params (Value :type Integer))
  (bind _asflying_saucer_game_mode (Utilities|Casting|CastToFlyingSaucerGameMode (Game|GetGameMode)))
  (Default|ChangePollutionEvent _asflying_saucer_game_mode Value))

(fn RemovePollution
  (params (Value :type Integer))
  (bind _asflying_saucer_game_mode (Utilities|Casting|CastToFlyingSaucerGameMode (Game|GetGameMode)))
  (Default|ChangePollutionEvent _asflying_saucer_game_mode (* Value -1)))

(fn SetPosition
  (params (Yaw :type Float%20%28single-precision%29) (Pitch :type Float%20%28single-precision%29) (Height :type Float%20%28single-precision%29))
  (Transformation|SetActorLocation (Class|KismetMathLibrary|CreateVectorfromYawPitch Yaw Pitch Height) true false)
  (Transformation|SetActorRotation (Math|Rotator|MakeRotfromZ (Transformation|GetActorLocation))))

(fn SetPositionBots
  (params (Yaw :type Float%20%28single-precision%29) (Pitch :type Float%20%28single-precision%29) (Height :type Float%20%28single-precision%29))
  (Transformation|SetActorLocation (Class|KismetMathLibrary|CreateVectorfromYawPitch Yaw Pitch Height) true false))