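; Base actor for spawnables such as ships and cars that move across the spherical Earth.
; Each tick it steps forward, line-traces from above toward the planet centre to snap onto Earth, and re-aligns up radially while preserving local rotation.
; Comparing hit distance with the game mode's WaterHeight makes ships on land and cars on water yaw randomly by small amounts.
; Helper functions place it by yaw/pitch/height and report pollution changes to FlyingSaucerGameMode.
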(event Custom|EventNewDirection
  ;[1 1 1] Choose random new direction to move in
  (Transformation|SetActorRotation (Math|Transform|TransformRotation (Math|Transform|MakeTransform "0, 0, 0" (Transformation|GetActorRotation)) (Math|Rotator|MakeRotator 0.0 0.0 (Math|Random|RandomFloatinRange 0.0 1e+01)))))

(event EventBeginPlay)

(event Collision|EventActorBeginOverlap
  (params (OtherActor :type Actor%20Object%20Reference)))

(event EventTick
  (params (DeltaSeconds :type Float%20%28single-precision%29))
  (bind _output_get (Variables|Default|Settmp_location (Transformation|GetActorLocation)))
  ;[1 1 1] Move the actor along the spherical surface in the direction of the forward vector
  (Transformation|SetActorLocation (Class|KismetMathLibrary|CreateVectorfromYawPitch (.Yaw (Math|Vector|GetYawPitchfromVector (+ _output_get (* (Transformation|GetActorForwardVector) (* (Variables|Default|GetSpeed) DeltaSeconds))))) (.Pitch (Math|Vector|GetYawPitchfromVector (+ _output_get (* (Transformation|GetActorForwardVector) (* (Variables|Default|GetSpeed) DeltaSeconds))))) (Math|Vector|VectorLength (+ _output_get (* (Transformation|GetActorForwardVector) (* (Variables|Default|GetSpeed) DeltaSeconds))))) false false)
  (bind _asflying_saucer_game_mode (Utilities|Casting|CastToFlyingSaucerGameMode (Game|GetGameMode)))
  ;[1 1 1] Measure distance to earth from a point above the target direction.
  (bind _outhit (Collision|LineTraceForObjects (* (Math|Vector|Normalize (+ _output_get (* (Transformation|GetActorForwardVector) (* (Variables|Default|GetSpeed) DeltaSeconds)))) (+ (Variables|/Game/Blueprints/FlyingSaucerGameMode.FlyingSaucerGameMode_C|GetWaterHeight _asflying_saucer_game_mode) (Variables|/Game/Blueprints/FlyingSaucerGameMode.FlyingSaucerGameMode_C|GetRayCastOffset _asflying_saucer_game_mode))) "0, 0, 0" (Utilities|Array|MakeArray "ObjectTypeQuery1") true 0 "None"))
  (Utilities|Casting|CastToEarth (.HitActor (Collision|BreakHitResult _outhit)))
  (Transformation|SetActorLocation (.Location (Collision|BreakHitResult _outhit)) false false)
  (Transformation|SetActorRotation (Math|Transform|TransformRotation (Math|Transform|MakeTransform "0, 0, 0" (Math|Rotator|MakeRotfromZ (.Location (Collision|BreakHitResult _outhit)))) (Math|Transform|InverseTransformRotation (Math|Transform|MakeTransform "0, 0, 0" (Math|Rotator|MakeRotfromZ _output_get)) (Transformation|GetActorRotation))))
  (bind _asflying_saucer_game_mode_2 (Utilities|Casting|CastToFlyingSaucerGameMode (Game|GetGameMode)))
  (Math|Float|CompareFloat (Math|Vector|VectorLength (.Location (Collision|BreakHitResult _outhit))) (Variables|/Game/Blueprints/FlyingSaucerGameMode.FlyingSaucerGameMode_C|GetWaterHeight _asflying_saucer_game_mode_2) ; If greater than the water height it's on land
    (:>
      ;[1 1 1] If a ship hits land it should turn
      (if (== (Utilities|GetClass self) "/Game/Blueprints/Spawnables/Ship.Ship_C")
        (CallFunction|EventNewDirection)))
    (:==
      ;[1 1 1] If a car hits water it should turn
      (if (== (Utilities|GetClass self) "/Game/Blueprints/Spawnables/Car.Car_C") :!label _label
        (CallFunction|EventNewDirection)))
    (:<
      (goto _label))))

(fn ConstructionScript)

(fn AddPollution
  (params (Value :type Integer))
  (bind _asflying_saucer_game_mode (Utilities|Casting|CastToFlyingSaucerGameMode (Game|GetGameMode)))
  (Default|ChangePollutionEvent _asflying_saucer_game_mode Value))

(fn RemovePollution
  (params (Value :type Integer))
  (bind _asflying_saucer_game_mode (Utilities|Casting|CastToFlyingSaucerGameMode (Game|GetGameMode)))
  (Default|ChangePollutionEvent _asflying_saucer_game_mode (* Value -1)))

(fn SetPosition
  (params (Yaw :type Float%20%28single-precision%29) (Pitch :type Float%20%28single-precision%29) (Height :type Float%20%28single-precision%29))
  (Transformation|SetActorLocation (Class|KismetMathLibrary|CreateVectorfromYawPitch Yaw Pitch Height) true false)
  (Transformation|SetActorRotation (Math|Rotator|MakeRotfromZ (Transformation|GetActorLocation))))

(fn SetPositionBots
  (params (Yaw :type Float%20%28single-precision%29) (Pitch :type Float%20%28single-precision%29) (Height :type Float%20%28single-precision%29))
  (Transformation|SetActorLocation (Class|KismetMathLibrary|CreateVectorfromYawPitch Yaw Pitch Height) true false))