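; Player-controlled flying saucer that moves over the surface of an invisible sphere centered on the world origin.
; BeginPlay derives starting yaw and pitch from the actor's location, and the vertical and horizontal input axes adjust them by fixed per-call steps.
; Tick converts the angles into a position at a fixed radius and aligns the saucer's Z axis outward from the origin.
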(event EventBeginPlay
  (bind _returnvalue (Transformation|GetActorLocation))
  (bind (_yaw _pitch) (Math|Vector|GetYawPitchfromVector _returnvalue))
  ;[1 1 1] Find the Pitch and Yaw of the ship at the beginning
  (Variables|Default|SetYaw _yaw)
  (Variables|Default|SetPitch _pitch))

(event Collision|EventActorBeginOverlap
  (params (OtherActor :type Actor%20Object%20Reference)))

(event EventTick
  (params (DeltaSeconds :type Float%20%28single-precision%29))
  (Transformation|SetActorLocation (Class|KismetMathLibrary|CreateVectorfromYawPitch (Variables|Default|GetYaw) (Variables|Default|GetPitch) 5.5e+02) false false)
  (Transformation|SetActorRotation (Math|Rotator|MakeRotfromZ (Transformation|GetActorLocation))))

(event Input|AxisEvents|InputAxisFlyingSaucerHorizontal
  (params (AxisValue :type Float%20%28single-precision%29))
  (Variables|Default|SetYaw (+ (Variables|Default|GetYaw) (* -0.5 AxisValue))))

(event Input|AxisEvents|InputAxisFlyingSaucerVertical
  (params (AxisValue :type Float%20%28single-precision%29))
  (Variables|Default|SetPitch (+ (Variables|Default|GetPitch) (* 0.5 AxisValue))))

(fn ConstructionScript)