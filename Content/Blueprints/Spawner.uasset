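; Spawner actor that populates the Earth with ships, oil rigs and cars while the flying saucer game mode is in Game Play.
; Tick spawns on a timer whose interval shrinks after each spawn down to a minimum.
; Placement line-traces from a random point above the globe to the Earth, orienting the actor to the radial direction with random yaw.
; Hit distance picks the class: ship or oil rig on lower surface, car on higher.
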(event EventBeginPlay)

(event Collision|EventActorBeginOverlap
  (params (OtherActor :type Actor%20Object%20Reference)))

(event EventTick
  (params (DeltaSeconds :type Float%20%28single-precision%29))
  (bind _asflying_saucer_game_mode (Utilities|Casting|CastToFlyingSaucerGameMode (Game|GetGameMode)))
  (switch Utilities|FlowControl|Switch|SwitchonEGameState (Variables|/Game/Blueprints/FlyingSaucerGameMode.FlyingSaucerGameMode_C|GetCurrentGameState _asflying_saucer_game_mode)
    (:NewEnumerator0
      ;[1 1 1] Spawn interval
      (bind _output_get (Variables|Default|SetCumulativeTime (+ DeltaSeconds (Variables|Default|GetCumulativeTime))))
      (Math|Float|CompareFloat _output_get (Variables|Default|GetSpawnInterval)
        (:>
          (Variables|Default|SetCumulativeTime (- _output_get (Variables|Default|GetSpawnInterval)))
          (bind (_hitdistance _hitlocation _transform) (CallFunction|GetRandomLocationandOrientation 5.5e+02))
          (Math|Float|CompareFloat _hitdistance 5e+01
            (:>
              (switch int (Math|Random|RandomInteger 2)
                (:0
                  (Game|SpawnActorfromClass "/Game/Blueprints/Spawnables/Ship.Ship_C" _transform "AlwaysSpawn" 0 0))
                (:1
                  (Game|SpawnActorfromClass "/Game/Blueprints/Spawnables/OilRig.OilRig_C" _transform "AlwaysSpawn" 0 0))))
            (:<
              (Game|SpawnActorfromClass "/Game/Blueprints/Spawnables/Car.Car_C" _transform "AlwaysSpawn" 0 0)))
          ;[1 1 1] Update the Spawn Interval
          (Math|Float|CompareFloat (Variables|Default|GetSpawnInterval) (Variables|Default|GetMinInterval)
            (:>
              (bind _output_get_2 (Variables|Default|SetSpawnInterval (- (Variables|Default|GetSpawnInterval) 0.01))))))))))

(fn ConstructionScript)

(fn GetRandomLocationandOrientation
  (params (Height :type Float%20%28single-precision%29))
  ;[1 1 1] Create and store random point in space
  (bind _output_get (Variables|Default|Settmp_rnd (Math|Random|RandomUnitVector)))
  ;[1 1 1] Measure distance to earth (from random point in space)
  (bind _outhit (Collision|LineTraceForObjects (* _output_get Height) "0, 0, 0" (Utilities|Array|MakeArray "ObjectTypeQuery1") true 0 "None"))
  (Utilities|Casting|CastToEarth (.HitActor (Collision|BreakHitResult _outhit)))
  (return (.Distance (Collision|BreakHitResult _outhit)) (.Location (Collision|BreakHitResult _outhit)) (Math|Transform|MakeTransform (.Location (Collision|BreakHitResult _outhit)) (Math|Transform|TransformRotation (Math|Transform|MakeTransform "0, 0, 0" (Math|Rotator|MakeRotfromZ _output_get)) (Math|Rotator|MakeRotator 0.0 0.0 (Math|Random|RandomFloatinRange 0.0 3.6e+02))))))