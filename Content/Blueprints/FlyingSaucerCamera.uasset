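; Flying saucer camera actor that becomes the view target, trails the player pawn and carries pollution fog planes.
; On BeginPlay it offsets the camera component by HeightOffset along the normalized player controller location.
; Each Tick it turns toward the world origin and lerps toward the pawn, scaled by delta time.
; UpdatePollution feeds the pollution ratio into two dynamic fog materials created in the construction script.
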(event Custom|UpdatePollution
  (params (pollution :type Integer) (maxpollution :type Integer))
  (bind _returnvalue (Math|Conversions|ToFloat(Integer) pollution))
  (bind _returnvalue_2 (Math|Conversions|ToFloat(Integer) maxpollution))
  (bind _returnvalue_3 (/ _returnvalue _returnvalue_2))
  ;[1 1 1] Update the Pollution Fog
  (Rendering|Material|SetScalarParameterValue (Variables|Default|GetDynamicMaterial1) "Pollution" _returnvalue_3 :!class /Script/Engine.MaterialInstanceDynamic)
  (Rendering|Material|SetScalarParameterValue (Variables|Default|GetDynamicMaterial2) "Pollution" _returnvalue_3 :!class /Script/Engine.MaterialInstanceDynamic))

(event EventBeginPlay
  ;[1 1 1] Set current camera
  (Game|Player|SetViewTargetwithBlend (Game|GetPlayerController 0) self 0.0 "VTBlend_Linear" 0.0 false)
  ;;[1 1 1] Set the camera location with CameraOffset
  (Transformation|SetRelativeLocation (Variables|Default|GetCamera) (* (Math|Vector|Normalize (Transformation|GetActorLocation (Game|GetPlayerController 0))) (Variables|Default|GetHeightOffset)) false false))

(event EventTick
  (params (DeltaSeconds :type Float%20%28single-precision%29))
  ;[1 1 1] Rotate the camera to look at the Origin
  (Transformation|SetActorRotation (Math|Rotator|FindLookatRotation (Transformation|GetActorLocation) (Math|Vector|VectorZero)))
  ;[1 1 1] Update the camera position by Lerping towards the Player
  (Transformation|SetActorLocation (Math|Vector|Lerp(Vector) (Transformation|GetActorLocation) (Transformation|GetActorLocation (Game|Player|GetPlayerPawn 0)) (* DeltaSeconds 3.0)) false false))

(fn ConstructionScript
  (bind _returnvalue (Rendering|Material|CreateDynamicMaterialInstance (Variables|Default|GetPlane) 0 "/Game/Blueprints/Materials/Fog_instance.Fog_instance" "None" :!class /Script/Engine.PrimitiveComponent))
  (Variables|Default|SetDynamicMaterial1 _returnvalue)
  (bind _returnvalue_2 (Rendering|Material|CreateDynamicMaterialInstance (Variables|Default|GetPlane1) 0 "/Game/Blueprints/Materials/Fog_front_nstance.Fog_front_nstance" "None" :!class /Script/Engine.PrimitiveComponent))
  (Variables|Default|SetDynamicMaterial2 _returnvalue_2))